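; BP_Pawn is a VR pawn with early scaffolding for grabbing objects with left and right hands.
; It sets eye-level tracking origin on BeginPlay and prints grip axis values and grab press/release events for debugging.
; Either grab press calls a shared FindNearestObjectToGrab, which only runs a Visibility box trace so far.
; The trace result is unused and nothing is attached or released yet.
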(event EventBeginPlay
  (Class|HeadMountedDisplayFunctionLibrary|SetTrackingOrigin "Eye"))

(event Collision|EventActorBeginOverlap
  (params (OtherActor :type Actor%20Object%20Reference)))

(event EventTick
  (params (DeltaSeconds :type Float%20%28single-precision%29)))

(event Input|ActionEvents|InputActionGrab_Left
  (params (Key :type Key%20Structure :default "None"))
  (:Pressed
    (Development|PrintString "Left Pressed")
    (CallFunction|FindNearestObjecttoGrab))
  (:Released
    (Development|PrintString "Left Released")))

(event Input|ActionEvents|InputActionGrab_Right
  (params (Key :type Key%20Structure :default "None"))
  (:Pressed
    (Development|PrintString "Right Pressed")
    (CallFunction|FindNearestObjecttoGrab))
  (:Released
    (Development|PrintString "Right Released")))

(event Input|AxisEvents|InputAxisGripAxis_Left
  (params (AxisValue :type Float%20%28single-precision%29))
  (Development|PrintString (Utilities|String|ToString(Float) AxisValue)))

(event Input|AxisEvents|InputAxisGripAxis_Right
  (params (AxisValue :type Float%20%28single-precision%29))
  (Development|PrintString (Utilities|String|ToString(Float) AxisValue)))

(fn ConstructionScript)

(fn FindNearestObjecttoGrab
  (Collision|BoxTraceByChannel "0, 0, 0" "0, 0, 0" "0, 0, 0" "0, 0, 0" "TraceTypeQuery1" false 0 "None"))